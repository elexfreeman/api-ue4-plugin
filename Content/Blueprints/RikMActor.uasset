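; RikMActor is an actor that drives an on-screen character search through RmApi and the RM_MainWiget UI.
; On BeginPlay it starts an initial "ric" query, binds the load-done event, and adds the widget to the viewport.
; Text committed in the widget triggers a new query.
; When loading completes, an event callback pushes the character array to the widget's list and refocuses its input.
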(event Custom|eventOnLoadCharDone_Event_0
  (Default|EventUpdateList (Variables|Default|GetmainWiget) (Variables|/Script/RikMortyApiPlg.RmApi|GetaChar (Variables|Default|GetRmApi)))
  (Default|EventSetFocusInput (Variables|Default|GetmainWiget)))

(event Custom|onTextCommit_Event_0
  (params (sText :type String))
  (Class|RmApi|FCharListCtrl (Variables|Default|GetRmApi) sText))

(event EventBeginPlay
  (Class|RmApi|FCharListCtrl (Variables|Default|GetRmApi) "ric")
  (EventDispatchers|AssignEventonLoadCharDone (Variables|Default|GetRmApi) (delegate Custom|eventOnLoadCharDone_Event_0))
  (bind _returnvalue (UserInterface|CreateWidget "/RikMortyApiPlg/Wigets/RM_MainWiget.RM_MainWiget_C"))
  (Variables|Default|SetmainWiget _returnvalue)
  (UserInterface|Viewport|AddtoViewport _returnvalue 0)
  (EventDispatchers|AssignOnTextCommit (Variables|Default|GetmainWiget) (delegate Custom|onTextCommit_Event_0)))

(event Collision|EventActorBeginOverlap
  (params (OtherActor :type Actor%20Object%20Reference)))

(event EventTick
  (params (DeltaSeconds :type Float%20%28single-precision%29)))

(fn ConstructionScript)